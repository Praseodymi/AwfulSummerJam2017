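; CivController is a controller that steers a civilian car (CivCar) around a network of CarNavNode actors.
; On BeginPlay it picks the node nearest its pawn.
; Each tick, once the pawn is within a squared reach distance, it hops to a random connected node and writes that location to the car's Target.
; Otherwise it draws a debug line at the current node; FindStartNode is an empty stub.
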(event EventBeginPlay
  (bind _returnvalue (Pawn|GetControlledPawn))
  (bind _returnvalue_2 (Transformation|GetActorLocation _returnvalue))
  (bind _outactors (Actor|GetAllActorsOfClass "/Game/Blueprints/CarNavNode.CarNavNode_C"))
  (Variables|Default|SettargetNode (Utilities|Array|Get(acopy) _outactors))
  (for _array_element _outactors
    (if (< (Math|Vector|VectorLengthSquared (- (Transformation|GetActorLocation _array_element) _returnvalue_2)) (Math|Vector|VectorLengthSquared (- (Transformation|GetActorLocation (Variables|Default|GettargetNode)) _returnvalue_2)))
      (Variables|Default|SettargetNode _array_element))))

(event EventTick
  (params (DeltaSeconds :type Float%20%28single-precision%29))
  (if (< (Math|Vector|VectorLengthSquared (- (Transformation|GetActorLocation (Variables|Default|GettargetNode)) (Transformation|GetActorLocation (Pawn|GetControlledPawn)))) (Variables|Default|GetnodeReachDistSqr))
    (bind _output_get (Variables|Default|SettargetNode (Utilities|Array|Get(acopy) (Variables|/Game/Blueprints/CarNavNode.CarNavNode_C|GetconnectedNodes (Variables|Default|GettargetNode)) (Math|Random|RandomInteger (Utilities|Array|Length (Variables|/Game/Blueprints/CarNavNode.CarNavNode_C|GetconnectedNodes (Variables|Default|GettargetNode)))))))
    (bind _asciv_car (Utilities|Casting|CastToCivCar (Pawn|GetControlledPawn)))
    (Variables|/Game/Blueprints/CivCar.CivCar_C|Settarget _asciv_car (Transformation|GetActorLocation _output_get))
    (else
      (Rendering|Debug|DrawDebugLine (Transformation|GetActorLocation (Variables|Default|GettargetNode)) (+ (Transformation|GetActorLocation (Variables|Default|GettargetNode)) "0,0.000000,100.000000") "(R=0.097860,G=0.000000,B=1.000000,A=1.000000)" 1e+01 3.0))))

(fn ConstructionScript)

(fn FindStartNode)