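; CivCar is an AI-style vehicle Blueprint that drives itself toward a Target location.
; Each Tick, it applies throttle while forward speed is below SpeedLimit and releases it otherwise.
; Steering input is the unscaled angle in degrees between the forward vector and the direction to Target, signed by a right-vector dot product.
; The file never sets Target and contains no braking or arrival logic.
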(event EventBeginPlay
  (|CallParentFunction))

(event Collision|EventActorBeginOverlap
  (params (OtherActor :type Actor%20Object%20Reference)))

(event EventTick
  (params (DeltaSeconds :type Float%20%28single-precision%29))
  (bind _returnvalue (Transformation|GetActorLocation))
  (bind _vehiclemovement (Variables|Default|GetVehicleMovement))
  (bind _target (Variables|Default|Gettarget))
  (bind _returnvalue_2 (- _target _returnvalue))
  (|CallParentFunction DeltaSeconds)
  (if (< (Class|WheeledVehicleMovementComponent|GetForwardSpeed _vehiclemovement) (Variables|Default|GetspeedLimit))
    (Class|WheeledVehicleMovementComponent|SetThrottleInput _vehiclemovement 5.0)
    (else
      (Class|WheeledVehicleMovementComponent|SetThrottleInput _vehiclemovement 0.0)))
  (Class|WheeledVehicleMovementComponent|SetSteeringInput _vehiclemovement (* (Math|Float|Sign(Float) (Math|Vector|DotProduct (Transformation|GetActorRightVector) _returnvalue_2)) (Class|KismetMathLibrary|DegAcos (/ (Math|Vector|DotProduct (Transformation|GetActorForwardVector) _returnvalue_2) (Math|Vector|VectorLength _returnvalue_2))))))

(fn ConstructionScript
  (|CallParentFunction))