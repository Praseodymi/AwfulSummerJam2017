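; TestCar is a Blueprint, apparently a test car, that tracks whether it is carrying goods.
; CollectGoods sets the HasGoods flag, DeliverGoods clears it, and GetGoods returns it.
; The event graph and construction script add no logic of their own, with Tick and construction only calling the parent.
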(event EventBeginPlay
  (|CallParentFunction))

(event Collision|EventActorBeginOverlap
  (params (OtherActor :type Actor%20Object%20Reference)))

(event EventTick
  (params (DeltaSeconds :type Float%20%28single-precision%29))
  (|CallParentFunction DeltaSeconds))

(fn ConstructionScript
  (|CallParentFunction))

(fn CollectGoods
  (Variables|Default|SethasGoods true)
  (return))

(fn DeliverGoods
  (Variables|Default|SethasGoods false)
  (return))

(fn GetGoods
  (return (Variables|Default|GethasGoods)))