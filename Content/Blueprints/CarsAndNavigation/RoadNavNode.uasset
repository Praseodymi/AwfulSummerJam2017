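; Road navigation node that links its two child CarNavNodes to those of other RoadNavNodes at BeginPlay, forming a graph for cars.
; Neighbors qualify when a line trace hits their Center and the navmesh path to it is straight.
; A 2D cross-product side test connects right-side child to right-side child along each link, giving directional lanes.
; On first Tick it destroys its Center and BlockingPlane helpers and stops ticking.
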(event EventBeginPlay
  (CallFunction|BuildNodeGraph))

(event Collision|EventActorBeginOverlap
  (params (OtherActor :type Actor%20Object%20Reference)))

(event EventTick
  (params (DeltaSeconds :type Float%20%28single-precision%29))
  (Components|DestroyComponent (Variables|Default|GetBlockingPlane))
  (Components|DestroyComponent (Variables|Default|GetCenter))
  (Actor|Tick|SetActorTickEnabled false))

(fn ConstructionScript)

(fn BuildNodeGraph
  (bind _center (Variables|Default|GetCenter))
  (bind _returnvalue (Transformation|GetWorldLocation _center))
  (bind _returnvalue_2 (Math|Conversions|ToVector2D(Vector) _returnvalue))
  (bind _results (CallFunction|GetVisibleNodes))
  (for _array_element _results
    (bind _result (CallFunction|IsRight _returnvalue_2 (Math|Conversions|ToVector2D(Vector) (Transformation|GetWorldLocation (Variables|RoadNavNode_C|GetCenter _array_element))) (Math|Conversions|ToVector2D(Vector) (Transformation|GetWorldLocation (Variables|Default|GetFirstNode)))))
    (bind _result_2 (CallFunction|IsRight _returnvalue_2 (Math|Conversions|ToVector2D(Vector) (Transformation|GetWorldLocation (Variables|RoadNavNode_C|GetCenter _array_element))) (Math|Conversions|ToVector2D(Vector) (Transformation|GetWorldLocation (Variables|RoadNavNode_C|GetFirstNode _array_element)))))
    (if _result
      (bind _ascar_nav_node (Utilities|Casting|CastToCarNavNode (Variables|/Script/Engine.ChildActorComponent|GetChildActor (Variables|Default|GetFirstNode))))
      (LocalVariables|SetrightNode _ascar_nav_node)
      (else
        (bind _ascar_nav_node_2 (Utilities|Casting|CastToCarNavNode (Variables|/Script/Engine.ChildActorComponent|GetChildActor (Variables|Default|GetSecondNode))))
        (LocalVariables|SetrightNode _ascar_nav_node_2)))
    (if _result_2
      (bind _ascar_nav_node_3 (Utilities|Casting|CastToCarNavNode (Variables|/Script/Engine.ChildActorComponent|GetChildActor (Variables|RoadNavNode_C|GetFirstNode _array_element))))
      (Utilities|Array|AddUnique (Variables|/Game/Blueprints/CarsAndNavigation/CarNavNode.CarNavNode_C|GetconnectedNodes (LocalVariables|GetrightNode)) _ascar_nav_node_3)
      (else
        (bind _ascar_nav_node_4 (Utilities|Casting|CastToCarNavNode (Variables|/Script/Engine.ChildActorComponent|GetChildActor (Variables|RoadNavNode_C|GetSecondNode _array_element))))
        (Utilities|Array|AddUnique (Variables|/Game/Blueprints/CarsAndNavigation/CarNavNode.CarNavNode_C|GetconnectedNodes (LocalVariables|GetrightNode)) _ascar_nav_node_4)))))

(fn IsRight
  (params (linePoint1 :type Vector%202D%20Structure) (linePoint2 :type Vector%202D%20Structure) (point :type Vector%202D%20Structure))
  (bind (_x _y) (Math|Vector2D|BreakVector2D linePoint1))
  (bind (_x_2 _y_2) (Math|Vector2D|BreakVector2D linePoint2))
  (bind (_x_3 _y_3) (Math|Vector2D|BreakVector2D point))
  (return (< 0.0 (- (* (- _x_2 _x) (- _y_3 _y)) (* (- _y_2 _y) (- _x_3 _x))))))

(fn GetVisibleNodes
  (bind _nodelist (LocalVariables|GetnodeList))
  (bind _outactors (Actor|GetAllActorsOfClass "RoadNavNode_C"))
  (for _array_element _outactors
    (bind _outhit (Collision|LineTraceForObjects (Transformation|GetWorldLocation (Variables|Default|GetCenter)) (Transformation|GetWorldLocation (Variables|RoadNavNode_C|GetCenter _array_element)) (Utilities|Array|MakeArray (Utilities|Enum|LiteralenumEObjectTypeQuery "ObjectTypeQuery1")) false 0 "None"))
    (if (== (.HitComponent (Collision|BreakHitResult _outhit)) (Variables|RoadNavNode_C|GetCenter _array_element))
      (bind _returnvalue (Class|NavigationSystem|FindPathtoLocationSynchronously (Transformation|GetWorldLocation (Variables|Default|GetCenter)) (Transformation|GetWorldLocation (Variables|RoadNavNode_C|GetCenter _array_element))))
      (if (<= (Utilities|Array|Length (Variables|/Script/Engine.NavigationPath|GetPathPoints _returnvalue)) 2)
        (Utilities|Array|AddUnique _nodelist _array_element))))
  (return _nodelist))