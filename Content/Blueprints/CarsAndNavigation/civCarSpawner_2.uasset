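; Civilian car spawner actor that keeps one CivCar alive at its location.
; On BeginPlay it spawns a CivCar at its transform, randomly flipping its own yaw 180 degrees first to vary the car's direction.
; Each Tick, once the owned car is no longer valid, it respawns one when the player pawn is between MinSpawnDistance and SpawnDistance, compared using squared distances.
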(event EventBeginPlay
  (if (Math|Random|RandomBool)
    _
    (else
      (Transformation|SetActorRotation (Math|Rotator|MakeRotator 0.0 0.0 (+ (.Yaw (Math|Rotator|BreakRotator (Transformation|GetActorRotation))) 1.8e+02)) true)))
  (bind _returnvalue (Game|SpawnActorfromClass "/Game/Blueprints/CarsAndNavigation/CivCar.CivCar_C" (Transformation|GetActorTransform) "AlwaysSpawn" 0 0))
  (Variables|Default|SetownedCar _returnvalue))

(event Collision|EventActorBeginOverlap
  (params (OtherActor :type Actor%20Object%20Reference)))

(event EventTick
  (params (DeltaSeconds :type Float%20%28single-precision%29))
  (bind _returnvalue (Game|Player|GetPlayerPawn 0))
  (bind _returnvalue_2 (Transformation|GetActorLocation))
  (bind _returnvalue_3 (Transformation|GetActorLocation _returnvalue))
  (bind _returnvalue_4 (- _returnvalue_2 _returnvalue_3))
  (bind _returnvalue_5 (Math|Vector|VectorLengthSquared _returnvalue_4))
  (if (Math|Boolean|ANDBoolean (not (Utilities|IsValid (Variables|Default|GetownedCar))) (< _returnvalue_5 (Math|Float|Square (Variables|Default|GetspawnDistance))) (> _returnvalue_5 (Math|Float|Square (Variables|Default|GetminSpawnDistance))))
    (if (Math|Random|RandomBool)
      _
      (else
        (Transformation|SetActorRotation (Math|Rotator|MakeRotator 0.0 0.0 (+ (.Yaw (Math|Rotator|BreakRotator (Transformation|GetActorRotation))) 1.8e+02)) true)))
    (bind _returnvalue_6 (Game|SpawnActorfromClass "/Game/Blueprints/CarsAndNavigation/CivCar.CivCar_C" (Transformation|GetActorTransform) "AlwaysSpawn" 0 0))
    (Variables|Default|SetownedCar _returnvalue_6)))

(fn ConstructionScript)