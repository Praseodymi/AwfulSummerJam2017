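; CarNavNode is a navigation graph node actor, apparently for cars, that links to other nodes through its ConnectedNodes array.
; Its logic is debug visualization only, with no pathfinding or movement.
; BeginPlay draws the node's display name at its location as a long-lived label.
; Tick draws a line to each connected node every frame, each lasting several seconds, so the lines overlap.
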(event EventBeginPlay
  (bind _self self)
  (Rendering|Debug|DrawDebugString (Transformation|GetActorLocation _self) (Utilities|GetDisplayName _self) _self "(R=0.509476,G=0.550000,B=0.000000,A=1.000000)" 1e+03))

(event Collision|EventActorBeginOverlap
  (params (OtherActor :type Actor%20Object%20Reference)))

(event EventTick
  (params (DeltaSeconds :type Float%20%28single-precision%29))
  (for _array_element (Variables|Default|GetconnectedNodes)
    (Rendering|Debug|DrawDebugLine :LineStart (Transformation|GetActorLocation self) :LineEnd (Transformation|GetActorLocation _array_element) :Duration 1e+01 :Thickness 2.0)))

(fn ConstructionScript)