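; Three-way road junction actor that cycles traffic light phases and lets the player knock its lights.
; Tick uses a latent Delay as the phase timer, stepping through looping Order and Delays arrays that sequence six Step components.
; Each change turns off every step's child point lights and mesh collision, then enables the selected step's lights and query-only collision.
; Player hits on West, North and South boxes push the matching light along the pawn's forward vector.
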(event OnComponentHit(BoxWest)
  (params (HitComponent :type Primitive%20Component%20Object%20Reference) (OtherActor :type Actor%20Object%20Reference) (OtherComp :type Primitive%20Component%20Object%20Reference) (NormalImpulse :type Vector :default "0, 0, 0") (Hit :type Hit%20Result%20Structure%20%28by%20ref%29))
  (bind _returnvalue (Game|Player|GetPlayerPawn 0))
  (if (== OtherActor _returnvalue)
    (Class|PrimitiveComponent|AddForceatLocationLocal (Variables|Default|GetWestLight) (* (Transformation|GetActorForwardVector _returnvalue) 10000) "0, 0, 0" "None")))

(event OnComponentHit(BoxNorth)
  (params (HitComponent :type Primitive%20Component%20Object%20Reference) (OtherActor :type Actor%20Object%20Reference) (OtherComp :type Primitive%20Component%20Object%20Reference) (NormalImpulse :type Vector :default "0, 0, 0") (Hit :type Hit%20Result%20Structure%20%28by%20ref%29))
  (bind _returnvalue (Game|Player|GetPlayerPawn 0))
  (if (== OtherActor _returnvalue)
    (Class|PrimitiveComponent|AddForceatLocationLocal (Variables|Default|GetNorthLight) (* (Transformation|GetActorForwardVector _returnvalue) 10000) "0, 0, 0" "None")))

(event OnComponentHit(BoxSouth)
  (params (HitComponent :type Primitive%20Component%20Object%20Reference) (OtherActor :type Actor%20Object%20Reference) (OtherComp :type Primitive%20Component%20Object%20Reference) (NormalImpulse :type Vector :default "0, 0, 0") (Hit :type Hit%20Result%20Structure%20%28by%20ref%29))
  (bind _returnvalue (Game|Player|GetPlayerPawn 0))
  (if (== OtherActor _returnvalue)
    (Class|PrimitiveComponent|AddForceatLocationLocal (Variables|Default|GetSouthLight) (* (Transformation|GetActorForwardVector _returnvalue) 10000) "0, 0, 0" "None")))

(event EventBeginPlay
  (bind _steps (Variables|Default|Getsteps))
  (Utilities|Array|SetArrayElem _steps 0 (Variables|Default|Getstep0) true)
  (Utilities|Array|SetArrayElem _steps 1 (Variables|Default|Getstep1) true)
  (Utilities|Array|SetArrayElem _steps 2 (Variables|Default|Getstep2) true)
  (Utilities|Array|SetArrayElem _steps 3 (Variables|Default|Getstep3) true)
  (Utilities|Array|SetArrayElem _steps 4 (Variables|Default|Getstep4) true)
  (Utilities|Array|SetArrayElem _steps 5 (Variables|Default|Getstep5) true))

(event Collision|EventActorBeginOverlap
  (params (OtherActor :type Actor%20Object%20Reference)))

(event EventTick
  (params (DeltaSeconds :type Float%20%28single-precision%29))
  (bind _steps (Variables|Default|Getsteps))
  (Utilities|FlowControl|Delay (Math|Conversions|ToFloat(Integer) (Utilities|Array|Get(acopy) (Variables|Default|Getdelays) (Variables|Default|GetcurrentIndex))))
  (for _array_element _steps
    (for _array_element_2 (Components|GetChildrenComponents _array_element true)
      (bind _asstatic_mesh_component (Utilities|Casting|CastToStaticMeshComponent _array_element_2)
        (:then
          (Collision|SetCollisionEnabled _asstatic_mesh_component "NoCollision"))
        (:CastFailed
          (bind _aspoint_light_component (Utilities|Casting|CastToPointLightComponent _array_element_2))
          (Rendering|SetVisibility _aspoint_light_component false true)))))
  (for _array_element_3 (Components|GetChildrenComponents (Utilities|Array|Get(acopy) _steps (Utilities|Array|Get(acopy) (Variables|Default|Getorder) (Variables|Default|GetcurrentIndex))) false)
    (bind _asstatic_mesh_component_2 (Utilities|Casting|CastToStaticMeshComponent _array_element_3)
      (:then
        (Collision|SetCollisionEnabled _asstatic_mesh_component_2 "QueryOnly"))
      (:CastFailed
        (bind _aspoint_light_component_2 (Utilities|Casting|CastToPointLightComponent _array_element_3))
        (Rendering|SetVisibility _aspoint_light_component_2 true true))))
  (if (> (+ (Variables|Default|GetcurrentIndex) 1) (Utilities|Array|LastIndex (Variables|Default|Getorder)))
    (Variables|Default|SetcurrentIndex 0)
    (else
      (Variables|Default|SetcurrentIndex (+ (Variables|Default|GetcurrentIndex) 1)))))

(fn ConstructionScript)