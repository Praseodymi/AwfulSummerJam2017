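; Controller for a police car that patrols road nodes and chases the player car when it carries goods or a pursuit is active.
; Each tick, a range check and line trace confirm sight, then a navigation path to the player replaces the car's Target points.
; Otherwise it queues random connected nodes ahead, and clears InPursuit while still within SearchTime of the last sighting, not after it expires.
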(event EventBeginPlay
  (|CallParentFunction)
  (Utilities|IsValid (Pawn|GetControlledPawn) :!label _label
    (:Is%20Valid
      (CallFunction|GetNewTargetNode)
      (bind _aspolice_car (Utilities|Casting|CastToPoliceCar (Pawn|GetControlledPawn)))
      (bind _output_get (Variables|Default|SetpoliceCarRef _aspolice_car))
      (Utilities|Array|Add (Variables|/Game/Blueprints/CarsAndNavigation/CivCar.CivCar_C|Gettarget _output_get) (Transformation|GetActorLocation (Utilities|Array|Get(acopy) (Variables|Default|GettargetNodes)))))
    (:Is%20Not%20Valid
      (Utilities|FlowControl|Delay 0.1)
      (goto _label))))

(event EventTick
  (params (DeltaSeconds :type Float%20%28single-precision%29))
  (bind _returnvalue (Game|Player|GetPlayerPawn 0))
  (bind _policecarref (Variables|Default|GetpoliceCarRef))
  (bind _targetnodes (Variables|Default|GettargetNodes))
  (bind _targetnodes_2 (Variables|Default|GettargetNodes))
  (bind _policecarref_2 (Variables|Default|GetpoliceCarRef))
  (bind _policecarref_3 (Variables|Default|GetpoliceCarRef))
  (bind _targetnodes_3 (Variables|Default|GettargetNodes))
  (bind _targetnodes_4 (Variables|Default|GettargetNodes))
  (bind _policecarref_4 (Variables|Default|GetpoliceCarRef))
  (bind _returnvalue_2 (Utilities|Array|Length _targetnodes_2))
  (bind _returnvalue_3 (Transformation|GetActorLocation _policecarref))
  (bind _returnvalue_4 (Transformation|GetActorLocation _returnvalue))
  (bind _output (Utilities|Array|Get(acopy) _targetnodes))
  (if (Utilities|IsValid _policecarref)
    (bind _asplayer_car (Utilities|Casting|CastToPlayerCar _returnvalue))
    (bind _hasgoods (Default|HasGoods _asplayer_car))
    (if (or _hasgoods (Variables|/Game/Blueprints/CarsAndNavigation/PoliceCar.PoliceCar_C|GetinPursuit (Variables|Default|GetpoliceCarRef)))
      (if (<= (Math|Vector|VectorLengthSquared (- _returnvalue_3 _returnvalue_4)) (Math|Float|Square (Variables|Default|GetsightDistance)))
        (bind _outhit (Collision|LineTraceForObjects (+ (* (Transformation|GetActorUpVector _policecarref) 5e+01) _returnvalue_3) (+ (* (Transformation|GetActorUpVector _returnvalue) 5e+01) _returnvalue_4) (Utilities|Array|MakeArray "ObjectTypeQuery2" "ObjectTypeQuery1" "ObjectTypeQuery3" "ObjectTypeQuery5") false (Utilities|Array|MakeArray _policecarref) "ForOneFrame"))
        (if (== (.HitActor (Collision|BreakHitResult _outhit)) _returnvalue)
          (Utilities|Array|Clear (Variables|Default|GettargetNodes))
          (bind _returnvalue_5 (Class|NavigationSystem|FindPathtoLocationSynchronously (Transformation|GetActorLocation (Variables|Default|GetpoliceCarRef)) (Transformation|GetActorLocation (Game|Player|GetPlayerPawn 0))))
          (Variables|/Game/Blueprints/CarsAndNavigation/CivCar.CivCar_C|Settarget _policecarref_3 (Variables|/Script/Engine.NavigationPath|GetPathPoints _returnvalue_5))
          (Variables|/Game/Blueprints/CarsAndNavigation/PoliceCar.PoliceCar_C|SetinPursuit _policecarref_3 true)
          (Variables|/Game/Blueprints/CarsAndNavigation/PoliceCar.PoliceCar_C|SetlastSeenPlayerTime _policecarref_3 (Utilities|Time|GetGameTimeinSeconds))
          (else
            (if (> (+ (Variables|/Game/Blueprints/CarsAndNavigation/PoliceCar.PoliceCar_C|GetsearchTime _policecarref_4) (Variables|/Game/Blueprints/CarsAndNavigation/PoliceCar.PoliceCar_C|GetlastSeenPlayerTime _policecarref_4)) (Utilities|Time|GetGameTimeinSeconds)) :!label _label
              (Variables|/Game/Blueprints/CarsAndNavigation/PoliceCar.PoliceCar_C|SetinPursuit _policecarref_4 false))
            (if (> (Utilities|Array|Length (Variables|/Game/Blueprints/CarsAndNavigation/CivCar.CivCar_C|Gettarget _policecarref_4)) 0)
              _
              (else
                (CallFunction|GetNewTargetNode)
                (Utilities|Array|Clear (Variables|/Game/Blueprints/CarsAndNavigation/CivCar.CivCar_C|Gettarget _policecarref_4))
                (Utilities|Array|Add (Variables|/Game/Blueprints/CarsAndNavigation/CivCar.CivCar_C|Gettarget _policecarref_4) (Transformation|GetActorLocation (Utilities|Array|Get(acopy) _targetnodes_2)))))
            (while (and (< _returnvalue_2 (Variables|Default|GetfutureNodes)) (> _returnvalue_2 0))
              (CallFunction|AddRandomConnectedNode)
              (Utilities|Array|Add (Variables|/Game/Blueprints/CarsAndNavigation/CivCar.CivCar_C|Gettarget (Variables|Default|GetpoliceCarRef)) (Transformation|GetActorLocation (Utilities|Array|Get(acopy) _targetnodes_4 (Utilities|Array|LastIndex _targetnodes_4)))))
            (if (Utilities|Array|IsValidIndex _targetnodes)
              (Utilities|IsValid _output
                (:Is%20Valid
                  (if (and (> (Utilities|Array|Length _targetnodes) 0) (< (Math|Vector|VectorLengthSquared (- (Transformation|GetActorLocation _output) (Transformation|GetActorLocation _policecarref_2))) (Math|Float|Square (Variables|/Game/Blueprints/CarsAndNavigation/CivCar.CivCar_C|GetnodeReachDist _policecarref_2))))
                    (Utilities|Array|RemoveIndex (Variables|Default|GettargetNodes))
                    (CallFunction|AddRandomConnectedNode)
                    (Utilities|Array|Add (Variables|/Game/Blueprints/CarsAndNavigation/CivCar.CivCar_C|Gettarget (Variables|Default|GetpoliceCarRef)) (Transformation|GetActorLocation (Utilities|Array|Get(acopy) _targetnodes_3 (Utilities|Array|LastIndex _targetnodes_3))))))))))
        (else
          (goto _label)))
      (else
        (goto _label)))))

(fn ConstructionScript
  (|CallParentFunction))