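; Civilian car spawner actor that spawns a CivCar at its own transform when the player pawn comes within SpawnDistance.
; Tick compares squared distance and spawns only if it has no valid OwnedCar and over three seconds have passed since its last spawn.
; Before each spawn it randomly turns itself 180 degrees in yaw, so cars can face either way, and spawns them regardless of collision.
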(event EventBeginPlay)

(event Collision|EventActorBeginOverlap
  (params (OtherActor :type Actor%20Object%20Reference)))

(event EventTick
  (params (DeltaSeconds :type Float%20%28single-precision%29))
  (if (> (- (Utilities|Time|GetGameTimeinSeconds) (Variables|Default|GetlastCheck)) 3.0)
    (if (not (Utilities|IsValid (Variables|Default|GetownedCar)))
      (if (< (Math|Vector|VectorLengthSquared (- (Transformation|GetActorLocation) (Transformation|GetActorLocation (Game|Player|GetPlayerPawn 0)))) (Math|Float|Square (Variables|Default|GetspawnDistance)))
        (Variables|Default|SetlastCheck (Utilities|Time|GetGameTimeinSeconds))
        (if (Math|Random|RandomBool)
          _
          (else
            (Transformation|SetActorRotation (Math|Rotator|MakeRotator 0.0 0.0 (+ (.Yaw (Math|Rotator|BreakRotator (Transformation|GetActorRotation))) 1.8e+02)) true)))
        (bind _returnvalue (Game|SpawnActorfromClass "/Game/Blueprints/CarsAndNavigation/CivCar.CivCar_C" (Transformation|GetActorTransform) "AlwaysSpawn" 0 0))
        (Variables|Default|SetownedCar _returnvalue)))))

(fn ConstructionScript)