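; NPC van that drives along a list of target nodes, despawning when too far from the player.
; Tick passes pursuit, search or normal speed limits to UpdateMovement.
; In normal driving, a forward trace brakes for components tagged brakeBlockingPlane; the no-hit branch swaps Started and SpeedLimit inputs.
; At zero Health it cuts throttle and expires shortly after, though collision damage measures a zero vector, so never applies.
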(event OnComponentHit(collisionBox)
  (params (HitComponent :type Primitive%20Component%20Object%20Reference) (OtherActor :type Actor%20Object%20Reference) (OtherComp :type Primitive%20Component%20Object%20Reference) (NormalImpulse :type Vector :default "0, 0, 0") (Hit :type Hit%20Result%20Structure%20%28by%20ref%29))
  (bind _returnvalue (Math|Vector|VectorLength "0, 0, 0"))
  (bind _returnvalue_2 (/ _returnvalue 1e+05))
  (if (not (Utilities|Array|ContainsItem (Variables|/Game/GUI/GameInstance.GameInstance_C|GetvehicleHitIgnore (Variables|Default|GetglobalState)) (Utilities|GetDisplayName OtherActor)))
    (if (> _returnvalue_2 1.0)
      (Variables|Default|Sethealth (- (Variables|Default|Gethealth) (Math|Float|Min(Float) _returnvalue_2 1e+01))))))

(event EventBeginPlay
  (|CallParentFunction)
  (bind _asgame_instance (Utilities|Casting|CastToGameInstance (Game|GetGameInstance)))
  (Audio|Components|Audio|SetVolumeMultiplier (Variables|Default|GetEngineSound) (Variables|/Game/GUI/GameInstance.GameInstance_C|GetsoundVolume _asgame_instance) :!class /Script/Engine.AudioComponent))

(event Collision|EventActorBeginOverlap
  (params (OtherActor :type Actor%20Object%20Reference)))

(event EventTick
  (params (DeltaSeconds :type Float%20%28single-precision%29))
  (bind _returnvalue (Transformation|GetActorLocation))
  (bind _speedlimit (Variables|Default|GetspeedLimit))
  (if (Utilities|IsValid (Pawn|GetController))
    (if (> (Variables|Default|Gethealth) 0.0)
      (if (> (Math|Vector|VectorLengthSquared (- (Transformation|GetActorLocation (Game|Player|GetPlayerPawn 0)) (Transformation|GetActorLocation))) (Math|Float|Square (Variables|Default|GetkeepAliveDistance)))
        (Actor|DestroyActor)
        (else
          (if (< (Math|Vector|VectorLengthSquared (- (Utilities|Array|Get(acopy) (Variables|Default|Gettarget)) (Transformation|GetActorLocation))) (Math|Float|Square (Variables|Default|GetnodeReachDist)))
            (Utilities|Array|RemoveIndex (Variables|Default|Gettarget))
            (Variables|Default|Setstarted (Utilities|Time|GetGameTimeinSeconds)))
          (if (Variables|Default|GetinPursuit)
            (CallFunction|UpdateMovement (Variables|Default|Getstarted) (Variables|Default|GetpursuitSpeedLimit) false)
            (elif (<= (- (Utilities|Time|GetGameTimeinSeconds) (Variables|Default|GetlastSeenPlayerTime)) (Variables|Default|GetsearchTime))
              (CallFunction|UpdateMovement (Variables|Default|Getstarted) (Variables|Default|GetsearchingSpeedLimit) false)
              (else
                (bind _outhit (Collision|LineTraceByChannel (+ _returnvalue "0,0.000000,50.000000") (+ _returnvalue (* (Transformation|GetActorForwardVector) 4e+02) "0,0.000000,50.000000") "TraceTypeQuery3" false 0 "ForOneFrame"))
                (if (Utilities|IsValid (.HitComponent (Collision|BreakHitResult _outhit)))
                  (CallFunction|UpdateMovement (Variables|Default|Getstarted) _speedlimit (Components|ComponentHasTag (.HitComponent (Collision|BreakHitResult _outhit)) "brakeBlockingPlane"))
                  (else
                    (CallFunction|UpdateMovement _speedlimit (Variables|Default|Getstarted) false))))))))
      (else
        (Utilities|FlowControl|DoOnce false
          (:Completed
            (Actor|SetLifeSpan 1e+01)
            (Class|WheeledVehicleMovementComponent|SetThrottleInput (Variables|Default|GetVehicleMovement) 0.0)))))))

(fn ConstructionScript
  (|CallParentFunction)
  (Variables|Default|SetlastSeenPlayerTime (- 0.0 (Variables|Default|GetsearchTime))))