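; Police car that follows a list of target points, switching between pursuit, search and patrol driving, and destroys itself when far from the player.
; Each tick it drops reached points and passes the current mode's speed limit to UpdateMovement.
; Only patrol brakes, when a forward trace hits a component tagged as a blocking plane.
; With no trace hit, patrol passes Started and SpeedLimit to UpdateMovement swapped.
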(event EventBeginPlay
  (|CallParentFunction))

(event Collision|EventActorBeginOverlap
  (params (OtherActor :type Actor%20Object%20Reference)))

(event EventTick
  (params (DeltaSeconds :type Float%20%28single-precision%29))
  (bind _returnvalue (Transformation|GetActorLocation))
  (bind _speedlimit (Variables|Default|GetspeedLimit))
  (if (Utilities|IsValid (Pawn|GetController))
    (bind _outhit (Collision|LineTraceByChannel (+ _returnvalue "0,0.000000,50.000000") (+ _returnvalue (* (Transformation|GetActorForwardVector) 4e+02) "0,0.000000,50.000000") "TraceTypeQuery3" false 0 "ForOneFrame"))
    (if (< (Math|Vector|VectorLengthSquared (- (Utilities|Array|Get(acopy) (Variables|Default|Gettarget)) (Transformation|GetActorLocation))) (Math|Float|Square (Variables|Default|GetnodeReachDist)))
      (Utilities|Array|RemoveIndex (Variables|Default|Gettarget))
      (Variables|Default|Setstarted (Utilities|Time|GetGameTimeinSeconds)))
    (if (Variables|Default|GetinPursuit)
      (CallFunction|UpdateMovement (Variables|Default|Getstarted) (Variables|Default|GetpursuitSpeedLimit) false)
      (elif (<= (- (Utilities|Time|GetGameTimeinSeconds) (Variables|Default|GetlastSeenPlayerTime)) (Variables|Default|GetsearchTime))
        (CallFunction|UpdateMovement (Variables|Default|Getstarted) (Variables|Default|GetsearchingSpeedLimit) false)
        (elif (Utilities|IsValid (.HitComponent (Collision|BreakHitResult _outhit)))
          (CallFunction|UpdateMovement (Variables|Default|Getstarted) _speedlimit (Components|ComponentHasTag (.HitComponent (Collision|BreakHitResult _outhit)) "brakeBlockingPlane"))
          (else
            (CallFunction|UpdateMovement _speedlimit (Variables|Default|Getstarted) false)))))
    (if (> (Math|Vector|VectorLengthSquared (- (Transformation|GetActorLocation (Game|Player|GetPlayerPawn 0)) (Transformation|GetActorLocation))) (Math|Float|Square (Variables|Default|GetkeepAliveDistance)))
      (Actor|DestroyActor))))

(fn ConstructionScript
  (|CallParentFunction)
  (Variables|Default|SetlastSeenPlayerTime (- 0.0 (Variables|Default|GetsearchTime))))