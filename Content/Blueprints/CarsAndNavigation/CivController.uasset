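; Controller for civilian cars that wanders them along the road node network by feeding target locations to the possessed CivCar.
; On BeginPlay it seeks the nearest RoadNavNode ahead and uses a side-of-line test to pick one of its two child CarNavNodes.
; Tick keeps a look-ahead queue of randomly connected nodes, replacing each one reached and otherwise drawing debug spheres.
; A quadratic Bezier helper is defined but not called here.
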(event EventBeginPlay
  (CallFunction|GetNewTargetNode)
  (bind _asciv_car (Utilities|Casting|CastToCivCar (Pawn|GetControlledPawn)))
  (Utilities|Array|Add (Variables|/Game/Blueprints/CarsAndNavigation/CivCar.CivCar_C|Gettarget _asciv_car) (Transformation|GetActorLocation (Utilities|Array|Get(acopy) (Variables|Default|GettargetNodes)))))

(event EventTick
  (params (DeltaSeconds :type Float%20%28single-precision%29))
  (bind _targetnodes (Variables|Default|GettargetNodes))
  (bind _targetnodes_2 (Variables|Default|GettargetNodes))
  (bind _targetnodes_3 (Variables|Default|GettargetNodes))
  (bind _asciv_car (Utilities|Casting|CastToCivCar (Pawn|GetControlledPawn)))
  (while (< (Utilities|Array|Length (Variables|Default|GettargetNodes)) (Variables|Default|GetfutureNodes))
    (CallFunction|AddRandomConnectedNode)
    (Utilities|Array|Add (Variables|/Game/Blueprints/CarsAndNavigation/CivCar.CivCar_C|Gettarget _asciv_car) (Transformation|GetActorLocation (Utilities|Array|Get(acopy) _targetnodes_3 (Utilities|Array|LastIndex _targetnodes_3)))))
  (if (< (Math|Vector|VectorLengthSquared (- (Transformation|GetActorLocation (Utilities|Array|Get(acopy) (Variables|Default|GettargetNodes))) (Transformation|GetActorLocation (Pawn|GetControlledPawn)))) (Variables|Default|GetnodeReachDistSqr))
    (Utilities|Array|RemoveIndex (Variables|Default|GettargetNodes))
    (CallFunction|AddRandomConnectedNode)
    (Utilities|Array|Add (Variables|/Game/Blueprints/CarsAndNavigation/CivCar.CivCar_C|Gettarget _asciv_car) (Transformation|GetActorLocation (Utilities|Array|Get(acopy) _targetnodes_2 (Utilities|Array|LastIndex _targetnodes_2))))
    (else
      (for (_array_element _array_index) _targetnodes
        (Rendering|Debug|DrawDebugSphere (Transformation|GetActorLocation _array_element) 1e+02 4 "(R=1.000000,G=0.000000,B=0.000000,A=1.000000)" 1.0 (Math|Conversions|ToFloat(Integer) (- (Utilities|Array|Length _targetnodes) _array_index)))))))

(fn ConstructionScript)

(fn GetBezierPoint
  (params (cp0 :type Vector) (cp1 :type Vector) (cp2 :type Vector) (t :type Float%20%28single-precision%29))
  (bind _returnvalue (Math|Float|Clamp(Float) t))
  (bind _returnvalue_2 (- 1.0 _returnvalue))
  (return (+ (* cp2 (Math|Float|Square _returnvalue)) (* cp1 (* 2.0 _returnvalue_2 _returnvalue)) (* cp0 (Math|Float|Square _returnvalue_2)))))

(fn GetNewTargetNode
  (bind _returnvalue (Pawn|GetControlledPawn))
  (bind _returnvalue_2 (Pawn|GetControlledPawn))
  (bind _targetnodes (Variables|Default|GettargetNodes))
  (bind _returnvalue_3 (Transformation|GetActorLocation _returnvalue_2))
  (bind _outactors (Actor|GetAllActorsOfClass "/Game/Blueprints/CarsAndNavigation/RoadNavNode.RoadNavNode_C"))
  (LocalVariables|SetnearestRoadNavNode (Utilities|Array|Get(acopy) _outactors))
  (for _array_element _outactors
    (if (> (Math|Vector|DotProduct (- (Transformation|GetActorLocation _array_element) (Transformation|GetActorLocation _returnvalue)) (Transformation|GetActorForwardVector _returnvalue)) 0.0)
      (if (< (Math|Vector|VectorLengthSquared (- (Transformation|GetActorLocation _array_element) _returnvalue_3)) (Math|Vector|VectorLengthSquared (- (Transformation|GetActorLocation (LocalVariables|GetnearestRoadNavNode)) _returnvalue_3)))
        (LocalVariables|SetnearestRoadNavNode _array_element))))
  (bind _result (Default|IsRight (LocalVariables|GetnearestRoadNavNode) (Math|Conversions|ToVector2D(Vector) (Transformation|GetActorLocation (Pawn|GetControlledPawn))) (Math|Conversions|ToVector2D(Vector) (Transformation|GetActorLocation (LocalVariables|GetnearestRoadNavNode))) (Math|Conversions|ToVector2D(Vector) (Transformation|GetActorLocation (Variables|/Script/Engine.ChildActorComponent|GetChildActor (Variables|/Game/Blueprints/CarsAndNavigation/RoadNavNode.RoadNavNode_C|GetFirstNode (LocalVariables|GetnearestRoadNavNode)))))))
  (if _result
    (bind _ascar_nav_node (Utilities|Casting|CastToCarNavNode (Variables|/Script/Engine.ChildActorComponent|GetChildActor (Variables|/Game/Blueprints/CarsAndNavigation/RoadNavNode.RoadNavNode_C|GetFirstNode (LocalVariables|GetnearestRoadNavNode)))))
    (Utilities|Array|Clear _targetnodes)
    (Utilities|Array|Add _targetnodes _ascar_nav_node)
    (else
      (bind _ascar_nav_node_2 (Utilities|Casting|CastToCarNavNode (Variables|/Script/Engine.ChildActorComponent|GetChildActor (Variables|/Game/Blueprints/CarsAndNavigation/RoadNavNode.RoadNavNode_C|GetSecondNode (LocalVariables|GetnearestRoadNavNode)))))
      (Utilities|Array|Clear _targetnodes)
      (Utilities|Array|Add _targetnodes _ascar_nav_node_2))))

(fn AddRandomConnectedNode
  (bind _targetnodes (Variables|Default|GettargetNodes))
  (bind _returnvalue (Utilities|Array|LastIndex _targetnodes))
  (bind _output (Utilities|Array|Get(acopy) _targetnodes _returnvalue))
  (bind _connectednodes (Variables|/Game/Blueprints/CarsAndNavigation/CarNavNode.CarNavNode_C|GetconnectedNodes _output))
  (Utilities|Array|Add _targetnodes (Utilities|Array|Get(acopy) _connectednodes (Math|Random|RandomInteger (Utilities|Array|Length _connectednodes)))))