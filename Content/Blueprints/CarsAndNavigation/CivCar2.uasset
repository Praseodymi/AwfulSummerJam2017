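; Civilian AI car that drives a waypoint list, despawns when too far from the player and expires shortly after Health runs out.
; Tick drops reached waypoints and feeds a forward trace for tagged brake planes into UpdateMovement.
; UpdateMovement steers or reverses by yaw to the waypoint, caps throttle over SpeedLimit and brakes if predicted travel overshoots the following waypoint.
; Collision damage tests a zero vector, so it never lowers Health.
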(event OnComponentHit(collisionBox)
  (params (HitComponent :type Primitive%20Component%20Object%20Reference) (OtherActor :type Actor%20Object%20Reference) (OtherComp :type Primitive%20Component%20Object%20Reference) (NormalImpulse :type Vector :default "0, 0, 0") (Hit :type Hit%20Result%20Structure%20%28by%20ref%29))
  (bind _returnvalue (Math|Vector|VectorLength "0, 0, 0"))
  (bind _returnvalue_2 (/ _returnvalue 1e+05))
  (if (not (Utilities|Array|ContainsItem (Variables|/Game/GUI/GameInstance.GameInstance_C|GetvehicleHitIgnore (Variables|Default|GetglobalState)) (Utilities|GetDisplayName OtherActor)))
    (if (> _returnvalue_2 1.0)
      (Variables|Default|Sethealth (- (Variables|Default|Gethealth) (Math|Float|Min(Float) _returnvalue_2 1e+01))))))

(event EventBeginPlay
  (|CallParentFunction)
  (bind _asgame_instance (Utilities|Casting|CastToGameInstance (Game|GetGameInstance)))
  (bind _output_get (Variables|Default|SetglobalState _asgame_instance))
  (Audio|Components|Audio|SetVolumeMultiplier (Variables|Default|GetEngineSound) (Variables|/Game/GUI/GameInstance.GameInstance_C|GetsoundVolume _output_get) :!class /Script/Engine.AudioComponent))

(event Collision|EventActorBeginOverlap
  (params (OtherActor :type Actor%20Object%20Reference)))

(event EventTick
  (params (DeltaSeconds :type Float%20%28single-precision%29))
  (bind _returnvalue (Transformation|GetActorLocation))
  (bind _speedlimit (Variables|Default|GetspeedLimit))
  (|CallParentFunction DeltaSeconds)
  (if (Utilities|IsValid (Pawn|GetController))
    (if (> (Variables|Default|Gethealth) 0.0)
      (if (> (Math|Vector|VectorLengthSquared (- (Transformation|GetActorLocation (Game|Player|GetPlayerPawn 0)) (Transformation|GetActorLocation))) (Math|Float|Square (Variables|Default|GetkeepAliveDistance)))
        (Actor|DestroyActor)
        (else
          (if (< (Math|Vector|VectorLengthSquared (- (Utilities|Array|Get(acopy) (Variables|Default|Gettarget)) (Transformation|GetActorLocation))) (Math|Float|Square (Variables|Default|GetnodeReachDist)))
            (Utilities|Array|RemoveIndex (Variables|Default|Gettarget))
            (Variables|Default|Setstarted (Utilities|Time|GetGameTimeinSeconds)))
          (bind _outhit (Collision|LineTraceByChannel (+ _returnvalue "0,0.000000,50.000000") (+ _returnvalue (* (Transformation|GetActorForwardVector) 4e+02) "0,0.000000,50.000000") "TraceTypeQuery3" false 0 "None"))
          (if (Utilities|IsValid (.HitComponent (Collision|BreakHitResult _outhit)))
            (CallFunction|UpdateMovement (Variables|Default|Getstarted) _speedlimit (Components|ComponentHasTag (.HitComponent (Collision|BreakHitResult _outhit)) "brakeBlockingPlane"))
            (else
              (CallFunction|UpdateMovement (Variables|Default|Getstarted) _speedlimit false)))))
      (else
        (Utilities|FlowControl|DoOnce false
          (:Completed
            (Actor|SetLifeSpan 1e+01)
            (Class|WheeledVehicleMovementComponent|SetThrottleInput (Variables|Default|GetVehicleMovement) 0.0)))))))

(fn ConstructionScript
  (|CallParentFunction))

(fn UpdateMovement
  (params (started :type Float%20%28single-precision%29) (speedLimit :type Float%20%28single-precision%29) (brakeOverride :type Boolean))
  (bind _returnvalue (Transformation|GetActorForwardVector))
  (bind _returnvalue_2 (Transformation|GetActorLocation))
  (bind _returnvalue_3 (Transformation|GetActorLocation))
  (bind _returnvalue_4 (Transformation|GetActorRotation))
  (bind _returnvalue_5 (Transformation|GetActorLocation))
  (bind _target (Variables|Default|Gettarget))
  (bind _vehiclemovement (Variables|Default|GetVehicleMovement))
  (bind _predictiontime (LocalVariables|GetpredictionTime))
  (bind _returnvalue_6 (Class|WheeledVehicleMovementComponent|GetForwardSpeed _vehiclemovement))
  (bind _output (Utilities|Array|Get(acopy) _target))
  (bind _returnvalue_7 (- _returnvalue_5 _output))
  (bind _returnvalue_8 (* _returnvalue _returnvalue_6))
  (bind _returnvalue_9 (Math|Rotator|FindLookatRotation _returnvalue_5 _output))
  (bind _returnvalue_10 (Math|Vector|VectorLength _returnvalue_7))
  (bind _returnvalue_11 (* _returnvalue_8 _predictiontime))
  (bind _returnvalue_12 (Math|Rotator|Delta(Rotator) _returnvalue_9 _returnvalue_4))
  (bind _yaw (Math|Rotator|BreakRotator _returnvalue_12))
  (bind _returnvalue_13 (+ _returnvalue_3 _returnvalue_11))
  (bind _returnvalue_14 (Math|Float|MapRangeUnclamped _yaw -3e+01 3e+01 -1.0 1.0))
  (bind _returnvalue_15 (Math|Float|InRange(Float) _yaw -9e+01 9e+01))
  (bind (_x _y) (Math|Vector|BreakVector _returnvalue_13))
  (bind _returnvalue_16 (Math|Integer|SelectInt 1 -1 _returnvalue_15))
  (bind _returnvalue_17 (Math|Float|SelectFloat _returnvalue_14 0.0 _returnvalue_15))
  (LocalVariables|Setdistance _returnvalue_10)
  (Class|WheeledVehicleMovementComponent|SetHandbrakeInput _vehiclemovement false)
  (Class|WheeledVehicleMovementComponent|SetBrakeInput _vehiclemovement 0.0)
  (Class|WheeledVehicleMovementComponent|SetSteeringInput _vehiclemovement (Math|Float|SelectFloat -1.0 (Math|Float|SelectFloat _returnvalue_17 _returnvalue_14 (and (not _returnvalue_15) (< _returnvalue_10 1e+03))) (== _returnvalue_17 0.0))) ; Update Steering Accordingly
  (LocalVariables|SetpredictedLocation (Math|Vector|MakeVector _x _y (.Z (Math|Vector|BreakVector _returnvalue_3))))
  (if (<= (Math|Vector|VectorLengthSquared (- _returnvalue_2 (LocalVariables|GetpredictedLocation))) (Math|Vector|VectorLengthSquared (- _returnvalue_2 (Utilities|Array|Get(acopy) (Variables|Default|Gettarget) 1))))
    (if brakeOverride
      (Class|WheeledVehicleMovementComponent|SetThrottleInput _vehiclemovement 0.0 :!label _label)
      (Class|WheeledVehicleMovementComponent|SetBrakeInput _vehiclemovement 1.0)
      (elif (<= (Class|WheeledVehicleMovementComponent|GetForwardSpeed _vehiclemovement) speedLimit)
        (Class|WheeledVehicleMovementComponent|SetThrottleInput _vehiclemovement (Math|Float|SelectFloat (* _returnvalue_16 (* (/ _returnvalue_10 (LocalVariables|Getdistance)) (Math|Float|Power (+ (* (LocalVariables|Getdistance) 2.5e-06) 1.0) (- (Utilities|Time|GetGameTimeinSeconds) started)))) (Math|Conversions|ToFloat(Integer) _returnvalue_16) (< (/ _returnvalue_10 (LocalVariables|Getdistance)) 0.5)))
        (else
          (Class|WheeledVehicleMovementComponent|SetThrottleInput _vehiclemovement (Math|Float|Min(Float) (Math|Float|SelectFloat (* _returnvalue_16 (* (/ _returnvalue_10 (LocalVariables|Getdistance)) (Math|Float|Power (+ (* (LocalVariables|Getdistance) 2.5e-06) 1.0) (- (Utilities|Time|GetGameTimeinSeconds) started)))) (Math|Conversions|ToFloat(Integer) _returnvalue_16) (< (/ _returnvalue_10 (LocalVariables|Getdistance)) 0.5)) 0.55)))))
    (else
      (goto _label))))