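; Environment Blueprint that places a row of child actors, likely power poles going by the asset name, along a spline.
; The construction script spaces NumberOfMeshes child actor components evenly by distance, dividing spline length by the count minus one so both ends get one.
; World spline locations are converted to actor-relative transforms, and OrientToSpline optionally rotates each child to the spline's direction at that point.
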(fn ConstructionScript
  (bind _number_of_meshes (Variables|Default|GetNumber%20of%20meshes))
  (bind _returnvalue (- _number_of_meshes 1))
  (if (> _number_of_meshes 0)
    (for _index (range 0 _returnvalue) ; Repeat loop for each mesh to add
      (bind _returnvalue_2 (AddComponent|AddChildActorComponent false (Math|Transform|MakeTransform (Math|Transform|InverseTransformLocation (Transformation|GetActorTransform) (Spline|GetLocationatDistanceAlongSpline (Variables|Default|GetSpline1) (* _index (/ (Spline|GetSplineLength (Variables|Default|GetSpline1)) (Math|Conversions|ToFloat(Integer) _returnvalue))) "World")) "0, 0, 0" "1.000000,1.000000,1.000000")))
      (if (Variables|Default|GetOrient%20to%20spline)
        (Transformation|SetWorldRotation _returnvalue_2 (Spline|GetRotationatDistanceAlongSpline (Variables|Default|GetSpline1) (* _index (/ (Spline|GetSplineLength (Variables|Default|GetSpline1)) (Math|Conversions|ToFloat(Integer) _returnvalue))) "World") false false) ; Rotate mesh to match direction of spline at its position
      ))))