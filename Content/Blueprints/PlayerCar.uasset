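; Player vehicle pawn with health, money, drink cargo, timed power-ups and HUD, pause and repair widgets.
; Paired DoOnce gates start power-ups from input; Tick expires them by timestamp: slow motion, halved damage, forward boost, huge mass, and an effectless fifth.
; Tick also keeps the minimap capture above the car, rotated with its heading.
; Hit impulses reduce health, skipping actors on the GameInstance ignore list.
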(event OnComponentHit(collisionBox)
  (params (HitComponent :type Primitive%20Component%20Object%20Reference) (OtherActor :type Actor%20Object%20Reference) (OtherComp :type Primitive%20Component%20Object%20Reference) (NormalImpulse :type Vector) (Hit :type Hit%20Result%20Structure%20%28by%20ref%29))
  (bind _returnvalue (Math|Vector|VectorLength NormalImpulse))
  (bind _returnvalue_2 (/ _returnvalue 1e+05))
  (if (not (Utilities|Array|ContainsItem (Variables|/Game/GUI/GameInstance.GameInstance_C|GetvehicleHitIgnore (Variables|Default|GetglobalState)) (Utilities|GetDisplayName OtherActor)))
    (if (> _returnvalue_2 1.0)
      (Variables|Default|Sethealth (- (Variables|Default|Gethealth) (Math|Float|Min(Float) (Variables|Default|Gethealth) (* (Math|Float|Min(Float) _returnvalue_2 1e+01) (Variables|Default|GetdamageMultiplier))))))))

(event EventBeginPlay
  (|CallParentFunction)
  (bind _returnvalue (UserInterface|CreateWidget "/Game/GUI/HUD.HUD_C"))
  (bind _output_get (Variables|Default|SetHUD%20Reference _returnvalue))
  (UserInterface|Viewport|AddtoViewport _output_get 0)
  (bind _returnvalue_2 (UserInterface|CreateWidget "/Game/GUI/PauseMenu.PauseMenu_C"))
  (bind _output_get_2 (Variables|Default|SetpauseMenu _returnvalue_2))
  (UserInterface|Viewport|AddtoViewport _output_get_2 0)
  (bind _returnvalue_3 (UserInterface|CreateWidget "/Game/GUI/Repair.Repair_C"))
  (bind _output_get_3 (Variables|Default|SetrepairMenuReference _returnvalue_3))
  (UserInterface|Viewport|AddtoViewport _output_get_3 0)
  (Widget|SetVisibility _output_get_3 "Collapsed")
  (bind _output_get_4 (Variables|Default|SetdrinkCount (Utilities|Array|MakeArray 0 0 0 0 0)))
  (for _index (range 0 (Utilities|Array|Length _output_get_4))
    (Default|UpdateCargoAmount (Variables|Default|GetHUD%20Reference) _index)
    (bind _asgame_instance (Utilities|Casting|CastToGameInstance (Game|GetGameInstance)))
    (bind _output_get_5 (Variables|Default|SetglobalState _asgame_instance))
    (Audio|Components|Audio|SetVolumeMultiplier (Variables|Default|GetEngineSound) (Variables|/Game/GUI/GameInstance.GameInstance_C|GetsoundVolume _output_get_5) :!class /Script/Engine.AudioComponent)
    (Variables|Default|SetminimapCameraVector (- (Transformation|GetWorldLocation (Variables|Default|GetMinimapCapture)) (Transformation|GetActorLocation)))
    (Variables|Default|Sethealth (Variables|/Game/GUI/GameInstance.GameInstance_C|GetplayerHealth (Variables|Default|GetglobalState)))
    (Variables|Default|Setmoney (Variables|/Game/GUI/GameInstance.GameInstance_C|GetplayerMoney (Variables|Default|GetglobalState)))))

(event EventTick
  (params (DeltaSeconds :type Float%20%28single-precision%29))
  (bind _postprocesssettings (Utilities|Struct|MakePostProcessSettings 0.0))
  (bind _postprocesssettings_2 (Utilities|Struct|MakePostProcessSettings 0.0))
  (bind _postprocesssettings_3 (Utilities|Struct|MakePostProcessSettings 1.0))
  (bind _postprocesssettings_4 (Utilities|Struct|MakePostProcessSettings 2.0))
  (bind _chasecamera (Variables|Default|GetChaseCamera))
  (bind _mesh (Variables|Character|GetMesh))
  (bind _internalcamera (Variables|Default|GetInternalCamera))
  (bind _chasecamera_2 (Variables|Default|GetChaseCamera))
  (bind _internalcamera_2 (Variables|Default|GetInternalCamera))
  (|CallParentFunction DeltaSeconds)
  (Transformation|SetWorldTransform (Variables|Default|GetMinimapCapture) (Math|Transform|MakeTransform (+ (Variables|Default|GetminimapCameraVector) (Transformation|GetActorLocation)) (Math|Rotator|MakeRotationfromAxes (Math|Vector|MakeVector 0.0 0.0 -1.0) (Transformation|GetActorRightVector) (Transformation|GetActorForwardVector))) false true)
  (for (_ _array_index) (Variables|Default|GetpowerLastCalled)
    (switch int _array_index
      (:0
        (bind _return (CallFunction|EffectHasExpired))
        (if _return
          (Utilities|FlowControl|DoOnce true
            (:Completed
              (Utilities|Time|SetGlobalTimeDilation 1.0)
              (Utilities|FlowControl|DoOnce false) ; enters at Reset
            ))))
      (:1
        (bind _return_2 (CallFunction|EffectHasExpired 1))
        (if _return_2
          (Utilities|FlowControl|DoOnce true
            (:Completed
              (Variables|/Script/Engine.CameraComponent|SetPostProcessSettings _chasecamera _postprocesssettings_2)
              (Variables|/Script/Engine.CameraComponent|SetPostProcessSettings _internalcamera _postprocesssettings_2)
              (Variables|Default|SetdamageMultiplier 1.0)
              (Utilities|FlowControl|DoOnce false) ; enters at Reset
            ))))
      (:2
        (bind _return_3 (CallFunction|EffectHasExpired 2))
        (if _return_3
          (Utilities|FlowControl|DoOnce true
            (:Completed
              (Variables|/Script/Engine.CameraComponent|SetPostProcessSettings _chasecamera_2 _postprocesssettings)
              (Variables|/Script/Engine.CameraComponent|SetPostProcessSettings _internalcamera_2 _postprocesssettings)
              (Variables|Default|SetboostValue 0.0)
              (Utilities|FlowControl|DoOnce false) ; enters at Reset
            ))))
      (:3
        (bind _return_4 (CallFunction|EffectHasExpired 3))
        (if _return_4
          (Utilities|FlowControl|DoOnce true
            (:Completed
              (Class|PrimitiveComponent|SetMassScale _mesh "None" 1.0)
              (Utilities|FlowControl|DoOnce false) ; enters at Reset
            ))))
      (:4
        (bind _return_5 (CallFunction|EffectHasExpired 4))
        (if _return_5
          (Utilities|FlowControl|DoOnce true
            (:Completed
              (Utilities|FlowControl|DoOnce false) ; enters at Reset
            ))))))
  (Transformation|SetActorLocation (+ (Transformation|GetActorLocation) (* (Transformation|GetActorForwardVector) (Variables|Default|GetboostValue))) true true))

(event Input|ActionEvents|InputActionPause
  (params (Key :type Key%20Structure :default "AnyKey"))
  (:Released
    (Default|Pause (Variables|Default|GetpauseMenu))))

(event Input|ActionEvents|InputActionPowerup3
  (params (Key :type Key%20Structure :default "AnyKey"))
  (bind _mesh (Variables|Character|GetMesh))
  (:Released
    (Utilities|FlowControl|DoOnce false
      (:Completed
        (Class|PrimitiveComponent|SetMassScale _mesh "None" 1e+06)
        (Utilities|Array|SetArrayElem (Variables|Default|GetpowerLastCalled) 3 (Utilities|Time|GetGameTimeinSeconds))
        (Utilities|FlowControl|DoOnce true) ; enters at Reset
      ))))

(event Input|ActionEvents|InputActionPowerup0
  (params (Key :type Key%20Structure :default "AnyKey"))
  (:Released
    (Utilities|FlowControl|DoOnce false
      (:Completed
        (Utilities|Time|SetGlobalTimeDilation 0.2)
        (Utilities|Array|SetArrayElem (Variables|Default|GetpowerLastCalled) 0 (Utilities|Time|GetGameTimeinSeconds))
        (Utilities|FlowControl|DoOnce true) ; enters at Reset
      ))))

(event Input|ActionEvents|InputActionPowerup1
  (params (Key :type Key%20Structure :default "AnyKey"))
  (bind _postprocesssettings (Utilities|Struct|MakePostProcessSettings 0.0))
  (bind _postprocesssettings_2 (Utilities|Struct|MakePostProcessSettings 1.0))
  (bind _chasecamera (Variables|Default|GetChaseCamera))
  (bind _internalcamera (Variables|Default|GetInternalCamera))
  (:Released
    (Utilities|FlowControl|DoOnce false
      (:Completed
        (Variables|/Script/Engine.CameraComponent|SetPostProcessSettings _chasecamera _postprocesssettings_2)
        (Variables|/Script/Engine.CameraComponent|SetPostProcessSettings _internalcamera _postprocesssettings_2)
        (Variables|Default|SetdamageMultiplier 0.5)
        (Utilities|Array|SetArrayElem (Variables|Default|GetpowerLastCalled) 1 (Utilities|Time|GetGameTimeinSeconds))
        (Utilities|FlowControl|DoOnce true) ; enters at Reset
      ))))

(event Input|ActionEvents|InputActionPowerup2
  (params (Key :type Key%20Structure :default "AnyKey"))
  (bind _postprocesssettings (Utilities|Struct|MakePostProcessSettings 0.0))
  (bind _postprocesssettings_2 (Utilities|Struct|MakePostProcessSettings 2.0))
  (bind _chasecamera (Variables|Default|GetChaseCamera))
  (bind _internalcamera (Variables|Default|GetInternalCamera))
  (:Released
    (Utilities|FlowControl|DoOnce false
      (:Completed
        (Variables|/Script/Engine.CameraComponent|SetPostProcessSettings _chasecamera _postprocesssettings_2)
        (Variables|/Script/Engine.CameraComponent|SetPostProcessSettings _internalcamera _postprocesssettings_2)
        (Variables|Default|SetboostValue 1e+01)
        (Utilities|Array|SetArrayElem (Variables|Default|GetpowerLastCalled) 2 (Utilities|Time|GetGameTimeinSeconds))
        (Utilities|FlowControl|DoOnce true) ; enters at Reset
      ))))

(event Input|ActionEvents|InputActionPowerup3
  (params (Key :type Key%20Structure :default "AnyKey"))
  (:Released
    (Utilities|FlowControl|DoOnce false
      (:Completed
        (Utilities|Array|SetArrayElem (Variables|Default|GetpowerLastCalled) 4 (Utilities|Time|GetGameTimeinSeconds))
        (Utilities|FlowControl|DoOnce true) ; enters at Reset
      ))))

(fn ConstructionScript
  (|CallParentFunction))

(fn AddMoney
  (params (m :type Integer))
  (Variables|Default|Setmoney (+ m (Variables|Default|Getmoney))))

(fn HasGoods
  (for _array_element (Variables|Default|GetdrinkCount)
    (bind _output_get (LocalVariables|SetdrinkCountTotal (+ _array_element (stale _output_get)))))
  (return (> _output_get 0)))

(fn EffectHasExpired
  (params (index :type Integer))
  (return (> (Utilities|Time|GetGameTimeinSeconds) (+ (Utilities|Array|Get(acopy) (Variables|Default|GetpowerLastCalled) index) (Utilities|Array|Get(acopy) (Variables|Default|GetpowerEffectLength) index)))))