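; ObjectiveSpawn is a placed spawn point for collect and drop objective actors, tied to the level's ObjectiveMaster.
; On BeginPlay it finds and caches the ObjectiveMaster, printing a warning unless exactly one exists.
; SpawnCollect and SpawnDrop spawn the matching actor at its transform and hand it a self reference.
; Its completion events forward to the master, passing this spawn point along.
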(event Custom|DropCompleteEvent
  (Default|DropCompleteEvent (Variables|Default|GetobjectiveMaster) self))

(event Custom|CollectCompleteEvent
  (Default|CollectCompeteEvent (Variables|Default|GetobjectiveMaster) self))

(event EventBeginPlay
  (bind _outactors (Actor|GetAllActorsOfClass "/Game/Blueprints/ObjectiveMaster.ObjectiveMaster_C"))
  (if (== (Utilities|Array|Length _outactors) 1)
    (Variables|Default|SetobjectiveMaster (Utilities|Array|Get(acopy) _outactors))
    (else
      (Development|PrintString "Uh oh! Multiple ObjectiveMasters present in scene!"))))

(event Collision|EventActorBeginOverlap
  (params (OtherActor :type Actor%20Object%20Reference)))

(event EventTick
  (params (DeltaSeconds :type Float%20%28single-precision%29)))

(fn ConstructionScript)

(fn SpawnCollect
  (bind _self self)
  (bind _returnvalue (Game|SpawnActorfromClass (Variables|Default|GetcollectActor) (Transformation|GetActorTransform _self) "AlwaysSpawn" 0 0))
  (Variables|/Game/Blueprints/CollectPoint.CollectPoint_C|SetobjectiveSpawn _returnvalue _self))

(fn SpawnDrop
  (bind _self self)
  (bind _returnvalue (Game|SpawnActorfromClass (Variables|Default|GetdropActor) (Transformation|GetActorTransform _self) "AlwaysSpawn" 0 0))
  (Variables|/Game/Blueprints/DropPoint.DropPoint_C|SetobjectiveSpawn _returnvalue _self))