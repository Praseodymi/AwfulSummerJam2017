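; Delivery drop point objective that sells the player car's cargo of one drink type when the car enters its sphere.
; On overlap it pays count times value, zeroes that cargo, updates the HUD, returns itself and its spawn to the ObjectiveMaster, then destroys itself.
; Each tick it moves its map icon toward its own location at fixed height, clamped to minimap radius around the player so distant points stay on the edge.
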(event OnComponentBeginOverlap(Sphere)
  (params (OverlappedComponent :type Primitive%20Component%20Object%20Reference) (OtherActor :type Actor%20Object%20Reference) (OtherComp :type Primitive%20Component%20Object%20Reference) (OtherBodyIndex :type Integer) (bFromSweep :type Boolean) (SweepResult :type Hit%20Result%20Structure%20%28by%20ref%29))
  (bind _goodtype (Variables|Default|GetgoodType))
  (bind _asplayer_car (Utilities|Casting|CastToPlayerCar OtherActor))
  (Default|AddMoney _asplayer_car (* (Utilities|Array|Get(acopy) (Variables|/Game/Blueprints/PlayerCar.PlayerCar_C|GetdrinkCount _asplayer_car) _goodtype) (Utilities|Array|Get(acopy) (Variables|/Game/Blueprints/PlayerCar.PlayerCar_C|GetdrinkValue _asplayer_car) _goodtype)))
  (Utilities|Array|SetArrayElem (Variables|/Game/Blueprints/PlayerCar.PlayerCar_C|GetdrinkCount _asplayer_car) _goodtype 0)
  (Default|UpdateCargoAmount (Variables|/Game/Blueprints/PlayerCar.PlayerCar_C|GetHUD%20Reference _asplayer_car) _goodtype)
  (Default|ReturnDropPoint (Variables|Default|GetobjectiveMaster) (Variables|Default|GetobjectiveSpawn) self)
  (Actor|DestroyActor))

(event EventBeginPlay
  (bind _outactors (Actor|GetAllActorsOfClass "/Game/Blueprints/Objective/ObjectiveMaster.ObjectiveMaster_C"))
  (Variables|Default|SetobjectiveMaster (Utilities|Array|Get(acopy) _outactors)))

(event EventTick
  (params (DeltaSeconds :type Float%20%28single-precision%29))
  (bind _returnvalue (Game|Player|GetPlayerPawn 0))
  (bind _returnvalue_2 (Transformation|GetActorLocation))
  (bind _returnvalue_3 (Transformation|GetActorLocation _returnvalue))
  (bind _returnvalue_4 (Math|Conversions|ToVector2D(Vector) _returnvalue_2))
  (bind _returnvalue_5 (Math|Conversions|ToVector2D(Vector) _returnvalue_3))
  (bind _returnvalue_6 (- _returnvalue_4 _returnvalue_5))
  (Transformation|SetWorldLocation (Variables|Default|GetMapIcon) (Math|Conversions|ToVector(Vector2D) (+ (* (Math|Vector2D|Normalize2D _returnvalue_6) (Math|Float|Min(Float) (Math|Vector2D|Vector2DLength _returnvalue_6) (Variables|Default|GetminimapSize))) _returnvalue_5) 2.5e+03) false false))

(fn ConstructionScript)