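; Objective manager that runs an endless collect-and-deliver loop over CollectSpawn and DropSpawn points placed in the level.
; On BeginPlay it gathers both sets of spawns and opens a random collect point for each of three good types.
; Returning a collect point spawns a drop point of the same good type, and returning that drop point spawns a new collect point.
; Active spawns leave the available pools until returned, preventing double use.
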(event EventBeginPlay
  (bind _outactors (Actor|GetAllActorsOfClass "/Game/Blueprints/Objective/CollectSpawn.CollectSpawn_C"))
  (Variables|Default|SetcollectPoints _outactors)
  (bind _outactors_2 (Actor|GetAllActorsOfClass "/Game/Blueprints/Objective/DropSpawn.DropSpawn_C"))
  (Variables|Default|SetdropPoints _outactors_2)
  (for _index (range 0 2)
    (CallFunction|SpawnCollectPoint _index)))

(event Collision|EventActorBeginOverlap
  (params (OtherActor :type Actor%20Object%20Reference)))

(event EventTick
  (params (DeltaSeconds :type Float%20%28single-precision%29)))

(fn ConstructionScript)

(fn ReturnCollectPoint
  (params (collectSpawn :type Collect%20Spawn%20Object%20Reference) (collectPoint :type Collect%20Point%20Object%20Reference))
  (Utilities|Array|RemoveItem (Variables|Default|GetcurrentCollectPoints) collectSpawn)
  (Utilities|Array|AddUnique (Variables|Default|GetcollectPoints) collectSpawn)
  (CallFunction|SpawnDropPoint (Variables|/Game/Blueprints/Objective/CollectPoint.CollectPoint_C|GetgoodType collectPoint)))

(fn ReturnDropPoint
  (params (dropSpawn :type Drop%20Spawn%20Object%20Reference) (dropPoint :type Drop%20Point%20Object%20Reference))
  (Utilities|Array|RemoveItem (Variables|Default|GetcurrentDropPoints) dropSpawn)
  (Utilities|Array|AddUnique (Variables|Default|GetdropPoints) dropSpawn)
  (CallFunction|SpawnCollectPoint (Variables|/Game/Blueprints/Objective/DropPoint.DropPoint_C|GetgoodType dropPoint)))

(fn SpawnCollectPoint
  (params (goodType :type Integer))
  (bind _collectpoints (Variables|Default|GetcollectPoints))
  (bind _currentcollectpoints (Variables|Default|GetcurrentCollectPoints))
  (bind _returnvalue (Utilities|Array|Add _currentcollectpoints (Utilities|Array|Get(acopy) _collectpoints (Math|Random|RandomInteger (Utilities|Array|Length _collectpoints)))))
  (Default|Spawn (Utilities|Array|Get(acopy) _currentcollectpoints _returnvalue) goodType)
  (Utilities|Array|RemoveItem _collectpoints (Utilities|Array|Get(acopy) _currentcollectpoints _returnvalue)))

(fn SpawnDropPoint
  (params (goodType :type Integer))
  (bind _droppoints (Variables|Default|GetdropPoints))
  (bind _currentdroppoints (Variables|Default|GetcurrentDropPoints))
  (bind _returnvalue (Utilities|Array|Add _currentdroppoints (Utilities|Array|Get(acopy) _droppoints (Math|Random|RandomInteger (Utilities|Array|Length _droppoints)))))
  (Default|Spawn (Utilities|Array|Get(acopy) _currentdroppoints _returnvalue) goodType)
  (Utilities|Array|RemoveItem _droppoints (Utilities|Array|Get(acopy) _currentdroppoints _returnvalue)))