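; CollectPoint is a pickup actor that refills one type of drink cargo on the player's car.
; When a PlayerCar overlaps it, it sets that GoodType's DrinkCount to the maximum and updates the HUD cargo amount.
; It then returns itself and its spawn to the ObjectiveMaster found at BeginPlay, and destroys itself.
; Every tick it draws its GoodType as debug text at its location.
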(event EventBeginPlay
  (bind _outactors (Actor|GetAllActorsOfClass "/Game/Blueprints/Objective/ObjectiveMaster.ObjectiveMaster_C"))
  (Variables|Default|SetobjectiveMaster (Utilities|Array|Get(acopy) _outactors)))

(event Collision|EventActorBeginOverlap
  (params (OtherActor :type Actor%20Object%20Reference))
  (bind _goodtype (Variables|Default|GetgoodType))
  (bind _asplayer_car (Utilities|Casting|CastToPlayerCar OtherActor))
  (Utilities|Array|SetArrayElem (Variables|/Game/Blueprints/PlayerCar.PlayerCar_C|GetdrinkCount _asplayer_car) _goodtype (Variables|/Game/Blueprints/PlayerCar.PlayerCar_C|GetdrinkCountMax _asplayer_car))
  (Default|UpdateCargoAmount (Variables|/Game/Blueprints/PlayerCar.PlayerCar_C|GetHUD%20Reference _asplayer_car) _goodtype)
  (Default|ReturnCollectPoint (Variables|Default|GetobjectiveMaster) (Variables|Default|GetobjectiveSpawn) self)
  (Actor|DestroyActor))

(event EventTick
  (params (DeltaSeconds :type Float%20%28single-precision%29))
  (Rendering|Debug|DrawDebugString (Transformation|GetActorLocation) (Utilities|String|ToString(Integer) (Variables|Default|GetgoodType)) 0 "(R=1.000000,G=1.000000,B=1.000000,A=1.000000)"))

(fn ConstructionScript)