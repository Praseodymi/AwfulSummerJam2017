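; ObjectiveMaster manages a repeating collect-and-drop objective loop across the level's ObjectiveSpawn actors.
; On BeginPlay it gathers them into a pool, and GenObjectivePair randomly chooses collect and drop spawns while removing two random entries.
; Removal and return each index randomly, so the returned spawns may differ from those removed.
; Collect completion re-adds its spawn to the pool; drop completion spawns a new pair before re-adding its own.
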(event Custom|CollectCompeteEvent
  (params (triggeredSpawn :type Objective%20Spawn%20Object%20Reference))
  (Utilities|Array|Add (Variables|Default|GetspawnPoints) triggeredSpawn))

(event Custom|DropCompleteEvent
  (params (triggeredSpawn :type Objective%20Spawn%20Object%20Reference))
  (bind _spawnpoints (Variables|Default|GetspawnPoints))
  (bind (_collectspawn _dropspawn) (CallFunction|GenObjectivePair _spawnpoints))
  (Default|SpawnCollect _collectspawn)
  (Default|SpawnDrop _dropspawn)
  (Utilities|Array|Add _spawnpoints triggeredSpawn))

(event EventBeginPlay
  (bind _outactors (Actor|GetAllActorsOfClass "/Game/Blueprints/ObjectiveSpawn.ObjectiveSpawn_C"))
  (bind _output_get (Variables|Default|SetspawnPoints _outactors))
  (bind (_collectspawn _dropspawn) (CallFunction|GenObjectivePair _output_get))
  (Default|SpawnCollect _collectspawn)
  (Default|SpawnDrop _dropspawn))

(event Collision|EventActorBeginOverlap
  (params (OtherActor :type Actor%20Object%20Reference)))

(event EventTick
  (params (DeltaSeconds :type Float%20%28single-precision%29)))

(fn ConstructionScript)

(fn GenObjectivePair
  (params (objArr :type Array%20of%20Objective%20Spawn%20Object%20References))
  (bind _returnvalue (Utilities|Array|Length objArr))
  (bind _returnvalue_2 (Math|Random|RandomInteger _returnvalue))
  (bind _returnvalue_3 (Math|Random|RandomInteger _returnvalue))
  (bind _output (Utilities|Array|Get(acopy) objArr _returnvalue_2))
  (bind _output_2 (Utilities|Array|Get(acopy) objArr _returnvalue_3))
  (Utilities|Array|RemoveItem objArr _output_2)
  (Utilities|Array|RemoveItem objArr _output)
  (return _output_2 _output))